(fn `Attach`
  (params (WorldLocation :type "Vector Structure"))
  (returns (Z_Offset :type "Float (double-precision)"))
  (bind _z (.z WorldLocation))
  (bind (_outhit _returnvalue) (`KismetSystemLibrary.LineTraceSingle` :`Start` WorldLocation :`End` (`KismetMathLibrary.MakeVector` (.x WorldLocation) (.y WorldLocation) (- _z 20000.0)) :`TraceChannel` "TraceTypeQuery1" :`bTraceComplex` true :`DrawDebugType` "ForDuration"))
  (if _returnvalue
    (return (- _z (.z (`.Location` (`GameplayStatics.BreakHitResult` _outhit)))))
    (else
      (return 0.0))))

(fn `Build`
  (bind _mesh (`self.Mesh`))
  (bind _f_scale (`self.F_Scale`))
  (bind _scalex (`self.ScaleX`))
  (bind _currentdistance (`self.CurrentDistance`))
  (bind _meshsize (`self.MeshSize`))
  (bind _spline (`self.Spline`))
  (bind _nextdistance (`self.NextDistance`))
  (bind _static_mesh_array (`self.Static_Mesh_Array`))
  (bind _outvalue (`self.Variation` (`self.Padding`) (`self.Padding_Variation`)))
  (bind (_returnvalue_origin _returnvalue_boxextent) (`KismetMathLibrary.BreakBoxSphereBounds` (`StaticMesh.GetBounds` (`|GetArrayItem` (`self.Static_Mesh_Array`) (`self.Index`)))))
  (bind (_returnvalue_origin_2 _returnvalue_boxextent_2) (`KismetMathLibrary.BreakBoxSphereBounds` (`StaticMesh.GetBounds` (`|GetArrayItem` (`self.Static_Mesh_Array`) (`self.Index`)))))
  (`self.ScaleFunc`)
  (set `self.Index` (`KismetMathLibrary.RandomIntegerInRange` 0 (- (`KismetArrayLibrary.Array_Length` (`self.Static_Mesh_Array`)) 1)))
  (set `self.MeshSize` (* (select `ESplineMeshAxis` (`self.In Forward Axis`) :`X` (.x _returnvalue_boxextent) :`Y` (.y _returnvalue_boxextent) :`Z` (.z _returnvalue_boxextent)) 2.0 (`self.F_Scale`)))
  (set `self.SplineLength` (`SplineComponent.GetSplineLength` (`self.Spline`)))
  (while (and (> (`self.SplineLength`) (`self.MeshSize`)) (!= (`KismetArrayLibrary.Array_Length` _static_mesh_array) 0) (`KismetArrayLibrary.Array_IsValidIndex` _static_mesh_array) (`KismetSystemLibrary.IsValid` (`|GetArrayItem` _static_mesh_array (`self.Index`))) (!= (`self.F_Scale`) 0.0))
    (set `self.NextDistance` (+ (`self.CurrentDistance`) (`self.MeshSize`)))
    (set `self.Start_Pos` (`SplineComponent.GetLocationAtDistanceAlongSpline` _spline _currentdistance "Local"))
    (set `self.End_Pos` (`SplineComponent.GetLocationAtDistanceAlongSpline` _spline _nextdistance "Local"))
    (set `self.Start Tangent` (`KismetMathLibrary.ClampVectorSize` (`SplineComponent.GetTangentAtDistanceAlongSpline` _spline _currentdistance "Local") _meshsize _meshsize))
    (set `self.EndTangent` (`KismetMathLibrary.ClampVectorSize` (`SplineComponent.GetTangentAtDistanceAlongSpline` _spline _nextdistance "Local") _meshsize _meshsize))
    (bind _returnvalue (`AddComponent|NODE_AddSplineMeshComponent-1`))
    (if (`self.Use Features?`)
      (bind _spline_2 (`self.FeatureFunc` _returnvalue))
      (set `self.Mesh` _spline_2)
      (else
        (set `self.Mesh` _returnvalue)))
    (`StaticMeshComponent.SetStaticMesh` _mesh (`|GetArrayItem` (`self.Static_Mesh_Array`) (`self.Index`)))
    (`SplineMeshComponent.SetStartScale` _mesh (`KismetMathLibrary.MakeVector2D` _scalex _f_scale) true)
    (`SplineMeshComponent.SetEndScale` _mesh (`KismetMathLibrary.MakeVector2D` _scalex _f_scale) true)
    (`SplineMeshComponent.SetForwardAxis` _mesh (`self.In Forward Axis`) true)
    (`PrimitiveComponent.SetCollisionEnabled` _mesh (`self.Collision`))
    (if (`self.UseTangent`)
      (`SplineMeshComponent.SetStartAndEnd` _mesh (`self.Start_Pos`) (`self.Start Tangent`) (`self.End_Pos`) (`self.EndTangent`) true)
      (else
        (`SplineMeshComponent.SetStartAndEnd` _mesh (`self.Start_Pos`) (0.0 0.0 0.0) (`self.End_Pos`) (0.0 0.0 0.0) true)))
    (if (`self.CanNegativePadding?`)
      (set `self.F_Padding` _outvalue)
      (else
        (set `self.F_Padding` (`KismetMathLibrary.Abs` _outvalue))))
    (set `self.CurrentDistance` (+ (`self.CurrentDistance`) (`self.MeshSize`) (`self.F_Padding`)))
    (set `self.Index` (`KismetMathLibrary.RandomIntegerInRange` 0 (- (`KismetArrayLibrary.Array_Length` (`self.Static_Mesh_Array`)) 1)))
    (set `self.SplineLength` (- (`self.SplineLength`) (+ (`self.MeshSize`) (`self.F_Padding`))))
    (`self.ScaleFunc`)
    (set `self.MeshSize` (* (select `ESplineMeshAxis` (`self.In Forward Axis`) :`X` (.x _returnvalue_boxextent_2) :`Y` (.y _returnvalue_boxextent_2) :`Z` (.z _returnvalue_boxextent_2)) 2.0 (`self.F_Scale`)))))

(fn `FeatureFunc`
  (params (`Spline Mesh` :type "SplineMeshComponent Object Reference"))
  (returns (Spline :type "SplineMeshComponent Object Reference"))
  (bind (_start_pos_x _start_pos_y _start_pos_z) (`KismetMathLibrary.BreakVector` (`self.Start_Pos`)))
  (bind (_end_pos_x _end_pos_y _end_pos_z) (`KismetMathLibrary.BreakVector` (`self.End_Pos`)))
  (bind (_start_tangent_x _start_tangent_y) (`KismetMathLibrary.BreakVector` (`self.Start Tangent`)))
  (bind (_endtangent_x _endtangent_y) (`KismetMathLibrary.BreakVector` (`self.EndTangent`)))
  (bind _returnvalue (/ (`self.F_Roll`) 57.32))
  (bind (_returnvalue_x _returnvalue_y _returnvalue_z) (`KismetMathLibrary.BreakVector` (`KismetMathLibrary.Vector_GetAbs` (`self.World_Offset_Variation`))))
  (bind _returnvalue_2 (+ (`SceneComponent.K2_GetComponentLocation` `Spline Mesh`) (`self.F_Loc`)))
  (bind (_returnvalue_x_2 _returnvalue_y_2 _returnvalue_z_2) (`KismetMathLibrary.BreakVector` (* (`KismetMathLibrary.MakeVector` _returnvalue_x _returnvalue_y _returnvalue_z) -1.0)))
  (bind _returnvalue_3 (/ (+ _start_pos_z _end_pos_z) 2.0))
  (if (`self.Plane`)
    (set `self.Start_Pos` (`KismetMathLibrary.MakeVector` _start_pos_x _start_pos_y _returnvalue_3))
    (set `self.End_Pos` (`KismetMathLibrary.MakeVector` _end_pos_x _end_pos_y _returnvalue_3))
    (set `self.Start Tangent` (`KismetMathLibrary.MakeVector` _start_tangent_x _start_tangent_y))
    (set `self.EndTangent` (`KismetMathLibrary.MakeVector` _endtangent_x _endtangent_y)))
  (set `self.F_Loc` (+ (`self.World_Offset`) (`KismetMathLibrary.MakeVector` (`KismetMathLibrary.RandomFloatInRange` _returnvalue_x_2 _returnvalue_x) (`KismetMathLibrary.RandomFloatInRange` _returnvalue_y_2 _returnvalue_y) (`KismetMathLibrary.RandomFloatInRange` _returnvalue_z_2 _returnvalue_z))))
  (if (`self.SnapToFloor?`)
    (`SceneComponent.K2_SetWorldLocation` `Spline Mesh` (+ (`KismetMathLibrary.MakeVector` (.x _returnvalue_2) (.y _returnvalue_2) (- (.z _returnvalue_2) (`self.Attach` (+ (`SplineComponent.GetLocationAtDistanceAlongSpline` (`self.Spline`) (/ (+ (`self.CurrentDistance`) (`self.NextDistance`)) 2.0) "World") (`self.F_Loc`))))) (`KismetMathLibrary.MakeVector` 0.0 0.0 (.z (`self.F_Loc`)))) false false)
    (else
      (`SceneComponent.K2_SetWorldLocation` `Spline Mesh` _returnvalue_2 false false)))
  (set `self.F_Roll` (`self.Variation` (`self.Rotation`) (`self.Rotation_Variation`)))
  (`SplineMeshComponent.SetStartRoll` `Spline Mesh` _returnvalue true)
  (`SplineMeshComponent.SetEndRoll` `Spline Mesh` _returnvalue true)
  (return `Spline Mesh`))

(fn `Scale_var`
  (params (Value :type "Float (double-precision)") (Variation :type "Float (double-precision)"))
  (returns (OutValue :type "Float (double-precision)"))
  (bind _returnvalue (`KismetMathLibrary.Abs` Variation))
  (return (`KismetMathLibrary.Abs` (+ Value (`KismetMathLibrary.RandomFloatInRange` (* _returnvalue -1.0) _returnvalue)))))

(fn `ScaleFunc`
  (bind _f_scale (`self.F_Scale`))
  (set `self.F_Scale` (`self.Scale_var` (`self.Scale`) (`self.Scale_Variation`)))
  (if (`self.RevertX`)
    (set `self.ScaleX` (* _f_scale -1.0))
    (else
      (set `self.ScaleX` _f_scale))))

(fn `UserConstructionScript`
  (if (`self.RealTimeBuild`)
    (`self.Build`)))

(fn `Variation`
  (params (Value :type "Float (double-precision)") (Variation :type "Float (double-precision)"))
  (returns (OutValue :type "Float (double-precision)"))
  (bind _returnvalue (`KismetMathLibrary.Abs` Variation))
  (return (+ Value (`KismetMathLibrary.RandomFloatInRange` (* _returnvalue -1.0) _returnvalue))))